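; Player pawn that accumulates a survival score and reacts to vehicle collisions with destroyable objects.
; Score grows each tick at a rate scaled from the game mode's move speed, updated through its speed-changed event.
; A VehicleTrigger overlap with a Destroyable registers a hit, then blocks further hits for a timed safe window.
; EndGame saves the rounded score as a high score through the game instance and opens ScreenLevel.
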(event OnComponentBeginOverlap(VehicleTrigger)
  (params (OverlappedComponent :type Primitive%20Component%20Object%20Reference) (OtherActor :type Actor%20Object%20Reference) (OtherComp :type Primitive%20Component%20Object%20Reference) (OtherBodyIndex :type Integer) (bFromSweep :type Boolean) (SweepResult :type Hit%20Result%20Structure%20%28by%20ref%29))
  (if (Variables|Default|GetbCanGetHit)
    (Utilities|Casting|CastToDestroyable OtherActor)
    (CallFunction|SetHitPossible false)
    (Class|PlayerPawn|RegisterHit)
    (Utilities|Time|SetTimerbyEvent (delegate Custom|RestartHitBox) (Variables|Default|GetSafeTime))))

(event Custom|RestartHitBox
  (CallFunction|SetHitPossible true))

(event Custom|UpdateScoreSpeed
  (params (NewSpeed :type Float%20%28double-precision%29))
  (Variables|Default|SetScoreSpeed (* NewSpeed 0.001)))

(event EventBeginPlay
  (bind _asbp_main_game_mode (Utilities|Casting|CastToBP_MainGameMode (Game|GetGameMode)))
  (Variables|Default|SetScoreSpeed (* (Variables|/Game/Configs/BP_MainGameMode.BP_MainGameMode_C|GetMoveSpeed _asbp_main_game_mode) 0.001))
  (EventDispatchers|BindEventtoSpeedChanged _asbp_main_game_mode (delegate Custom|UpdateScoreSpeed)))

(event Collision|EventActorBeginOverlap
  (params (OtherActor :type Actor%20Object%20Reference)))

(event EventTick
  (params (DeltaSeconds :type Float%20%28single-precision%29))
  (Variables|Default|SetScore (+ (Variables|Default|GetScore) (* DeltaSeconds (Variables|Default|GetScoreSpeed)))))

(event EventEndGame
  (bind _asode_to_design_instance (Utilities|Casting|CastToOdeToDesignInstance (Game|GetGameInstance)))
  (Class|OdetoDesignInstance|SaveHighScore _asode_to_design_instance (Math|Conversions|ToFloat(Integer) (Math|Float|Round (Variables|Default|GetScore))))
  (Game|OpenLevel(byName) "ScreenLevel"))

(fn ConstructionScript)

(fn SetHitPossible
  (params (bCanBeHit :type Boolean))
  (bind _output_get (Variables|Default|SetbCanGetHit bCanBeHit))
  (if _output_get
    _))